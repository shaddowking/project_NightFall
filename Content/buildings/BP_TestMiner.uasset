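; BP_TestMiner is a test miner building made of six cube meshes, with visual states for placement and construction.
; SetupGhost applies a ghost material and disables collision on all cubes.
; EditCanBuildColor swaps every cube between can-build and can't-build materials to show placement validity.
; SetupCreatedBuilding applies the body material, gives Cube1 its own distinct material, and restores query and physics collision.
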(event EventEditCanBuildColor
  (params (CanBuild :type Boolean))
  (bind _cube (Variables|Default|GetCube))
  (if CanBuild
    (Rendering|Material|SetMaterial _cube 0 "/Game/turrets/MI_CanBuild.MI_CanBuild")
    (else
      (Rendering|Material|SetMaterial _cube 0 "/Game/turrets/MI_CantBuild.MI_CantBuild"))))

(event EventSetupGhost
  (Rendering|Material|SetMaterial (Variables|Default|GetCube1) 0 "/Game/turrets/M_GhostMaterial.M_GhostMaterial")
  (Rendering|Material|SetMaterial (Variables|Default|GetCube) 0 "/Game/turrets/M_GhostMaterial.M_GhostMaterial")
  (Collision|SetCollisionEnabled (Variables|Default|GetCube) "NoCollision"))

(event EventSetupCreatedBuilding
  (Rendering|Material|SetMaterial (Variables|Default|GetCube1) 0 "/Game/enemy/demo_Materials/M_Demo_Dead.M_Demo_Dead")
  (Rendering|Material|SetMaterial (Variables|Default|GetCube) 0 "/Game/turrets/Light_Turret/M_Body.M_Body")
  (Collision|SetCollisionEnabled (Variables|Default|GetCube) "QueryAndPhysics"))

(fn ConstructionScript)