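; Cargo grid Blueprint, named as a 2x2 variant, whose event graph holds only debug and test helpers.
; DebugCargoGrid draws a slot-sized box at a given position.
; AddBox spawns a test box as the current cargo box, then calls SnapBoxToGrid and PlaceBox, which are defined outside this file.
; BeginPlay is empty, and a timed chain of repeated AddBox calls is left disconnected.
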(event Collision|EventActorBeginOverlap
  (params (OtherActor :type Actor%20Object%20Reference)))

(event EventTick
  (params (DeltaSeconds :type Float%20%28single-precision%29)))

(event EventDebugCargoGrid
  (params (pos :type Vector :default "0, 0, 0"))
  (Rendering|Debug|DrawDebugBox pos (Math|Conversions|ToVector(Float) (/ (Variables|Default|GetSlotSize) 2.0)) "(R=0.000000,G=0.000000,B=0.000000,A=1.000000)" "0, 0, 0" 5e+01 5.0))

(event EventBeginPlay)

(event EventAddBox
  ;[0.15 0.15 0.15 0.5] Debug Testing
  (bind _returnvalue (Game|SpawnActorfromClass "/Game/CargoGrids/TestBox.TestBox_C" (Math|Transform|MakeTransform "0, 0, 0" "0, 0, 0" "1.000000,1.000000,1.000000") "Undefined" "MultiplyWithRoot" 0 0))
  (Variables|Default|SetCurrentCargoBox _returnvalue)
  (Class|CargoGrid|SnapBoxtoGrid)
  (Class|CargoGrid|PlaceBox))

(fn ConstructionScript)