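; BP_LightTurret is a buildable light turret that handles the visual side of building placement.
; Setup events switch its base, gun and head between a ghost material without base collision and final materials with base collision restored.
; EditCanBuildColor tints all three meshes to show whether placement is valid.
; Two helper events draw debug spheres and lines; no targeting or firing logic is in these graphs.
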(event EventBeginPlay)

(event Collision|EventActorBeginOverlap
  (params (OtherActor :type Actor%20Object%20Reference)))

(event EventEditCanBuildColor
  (params (CanBuild :type Boolean))
  (if CanBuild
    (Rendering|Material|SetMaterial (Variables|Default|GetTurretBase) 0 "/Game/turrets/MI_CanBuild.MI_CanBuild")
    (Rendering|Material|SetMaterial (Variables|Default|Getgun) 0 "/Game/turrets/MI_CanBuild.MI_CanBuild")
    (Rendering|Material|SetMaterial (Variables|Default|Gethead) 0 "/Game/turrets/MI_CanBuild.MI_CanBuild")
    (else
      (Rendering|Material|SetMaterial (Variables|Default|GetTurretBase) 0 "/Game/turrets/MI_CantBuild.MI_CantBuild")
      (Rendering|Material|SetMaterial (Variables|Default|Getgun) 0 "/Game/turrets/MI_CantBuild.MI_CantBuild")
      (Rendering|Material|SetMaterial (Variables|Default|Gethead) 0 "/Game/turrets/MI_CantBuild.MI_CantBuild"))))

(event EventSetupGhost
  (Rendering|Material|SetMaterial (Variables|Default|GetTurretBase) 0 "/Game/turrets/M_GhostMaterial.M_GhostMaterial")
  (Collision|SetCollisionEnabled (Variables|Default|GetTurretBase) "NoCollision"))

(event EventSetupCreatedBuilding
  (Rendering|Material|SetMaterial (Variables|Default|GetTurretBase) 0 "/Game/turrets/Light_Turret/M_Body.M_Body")
  (Rendering|Material|SetMaterial (Variables|Default|Getgun) 0 "/Game/enemy/demo_Materials/M_Demo_Normal.M_Demo_Normal")
  (Rendering|Material|SetMaterial (Variables|Default|Gethead) 0 "/Game/enemy/demo_Materials/M_Demo_Dead.M_Demo_Dead")
  (Collision|SetCollisionEnabled (Variables|Default|GetTurretBase) "QueryAndPhysics"))

(event EventDebugTarget
  (params (targetLocation :type Vector :default "0, 0, 0"))
  (Rendering|Debug|DrawDebugSphere targetLocation 1e+02 12 "(R=0.000000,G=0.000000,B=0.000000,A=1.000000)" 0.0 1e+01))

(event EventDrawDebugLine
  (params (A :type Vector :default "0, 0, 0") (B :type Vector :default "0, 0, 0"))
  (Rendering|Debug|DrawDebugLine A B "(R=0.000000,G=0.000000,B=0.000000,A=1.000000)" 0.0 1e+01))

(fn ConstructionScript)