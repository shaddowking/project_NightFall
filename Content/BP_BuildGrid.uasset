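; BP_BuildGrid is a build grid actor that shows the extents of its cell-based volume with three axis arrows.
; The construction script sizes the X, Y and Z arrows as cell size times the grid count on that axis.
; A DebugBuildGrid event exists but is empty, with its debug box draw left disconnected, and the file has no active runtime logic.
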(event EventBeginPlay)

(event Collision|EventActorBeginOverlap
  (params (OtherActor :type Actor%20Object%20Reference)))

(event EventTick
  (params (DeltaSeconds :type Float%20%28single-precision%29)))

(event EventDebugBuildGrid
  (params (pos :type Vector :default "0, 0, 0") (extend :type Float%20%28single-precision%29)))

(fn ConstructionScript
  (bind _cellsize (Variables|Default|GetCellSize))
  (Variables|/Script/Engine.ArrowComponent|SetArrowLength (Variables|Default|GetArrowX) (Math|Conversions|ToFloat(Integer) (* _cellsize (Variables|Default|GetGrid_X))))
  (Variables|/Script/Engine.ArrowComponent|SetArrowLength (Variables|Default|GetArrowZ) (Math|Conversions|ToFloat(Integer) (* _cellsize (Variables|Default|GetGrid_Z))))
  (Variables|/Script/Engine.ArrowComponent|SetArrowLength (Variables|Default|GetArrowY) (Math|Conversions|ToFloat(Integer) (* _cellsize (Variables|Default|GetGrid_Y)))))